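; BP_InfiniteTerrainGameMode is the game mode for an endless tiled terrain, handling tile spawning and score.
; On BeginPlay it fills a nav mesh bounds volume pool and spawns an initial batch of BP_Tile actors.
; SpawnTile hands each tile the pool, then stores its attach location as the next spawn transform, chaining tiles end to end.
; NewTileConquered increments the score, which GetScore returns.
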(event EventBeginPlay
  (Class|InfiniteTerrainGameMode|PopulateBoundsVolumePool)
  (for _index (range 0 3)
    (CallFunction|SpawnTile)))

(event EventTick
  (params (DeltaSeconds :type Float%20%28single-precision%29)))

(fn ConstructionScript)

(fn SpawnTile
  (bind _returnvalue (Game|SpawnActorfromClass "/Game/Dynamic/Core/Procedurals/Tile/BP_Tile.BP_Tile_C" (Variables|Default|GetNextTile) "Undefined" 0 0))
  (Class|Tile|SetPool _returnvalue (Variables|Default|GetNavMeshBoundsVolumePool))
  (bind _attachtransform (Default|GetAttachLocation _returnvalue))
  (Variables|Default|SetNextTile _attachtransform)
  (return))

(fn NewTileConquered
  (Math|Integer|IncrementInt (Variables|Default|GetScore)
    (:%20%20
      (return))))

(fn GetScore
  (return (Variables|Default|GetScore)))